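; Spline actor that lays two parallel lines of cones, yellow and blue, along a path, rebuilt in the construction script and on BeginPlay.
; GenerarConos clears both instanced mesh components, then adds evenly spaced instances offset to either side of PathSpline along its right vector.
; All cones take the rotation at the spline's start.
; The blue loop is nested inside the yellow loop, so blue instances repeat for every yellow cone.
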(event EventBeginPlay
  (CallFunction|GenerarConos))

(event Collision|EventActorBeginOverlap
  (params (OtherActor :type Actor%20Object%20Reference)))

(fn ConstructionScript
  (CallFunction|GenerarConos))

(fn GenerarConos
  (bind _pathspline (Variables|Default|GetPathSpline))
  (bind _pathspline_2 (Variables|Default|GetPathSpline))
  (bind _returnvalue (Spline|GetRotationatDistanceAlongSpline _pathspline_2 0.0 "Local"))
  (Components|InstancedStaticMesh|ClearInstances (Variables|Default|GetISM_ConoAmarillo))
  (Components|InstancedStaticMesh|ClearInstances (Variables|Default|GetISM_ConoAzul))
  (for _index (range 0 (- (Variables|Default|GetNumeroDeConosNaranjas) 1))
    (Components|InstancedStaticMesh|AddInstance (Variables|Default|GetISM_ConoAmarillo) (Math|Transform|MakeTransform (- (Spline|GetLocationatDistanceAlongSpline _pathspline (+ (* (Variables|Default|GetSepracionEntreConos) (Math|Conversions|ToFloat(Integer) _index)) 0.01) "Local") (* (Class|SplineComponent|GetRightVectoratDistanceAlongSpline _pathspline (+ (* (Variables|Default|GetSepracionEntreConos) (Math|Conversions|ToFloat(Integer) _index)) 0.01) "Local") (Variables|Default|GetSeparacionEntreLineas))) _returnvalue))
    (for _index_2 (range 0 (- (Variables|Default|GetNumeroDeConosAzules) 1))
      (Components|InstancedStaticMesh|AddInstance (Variables|Default|GetISM_ConoAzul) (Math|Transform|MakeTransform (+ (Spline|GetLocationatDistanceAlongSpline _pathspline_2 (+ (* (Variables|Default|GetSepracionEntreConos) (Math|Conversions|ToFloat(Integer) _index_2)) 0.01) "Local") (* (Class|SplineComponent|GetRightVectoratDistanceAlongSpline _pathspline_2 (+ (* (Variables|Default|GetSepracionEntreConos) (Math|Conversions|ToFloat(Integer) _index_2)) 0.01) "Local") (Variables|Default|GetSeparacionEntreLineas))) _returnvalue)))))