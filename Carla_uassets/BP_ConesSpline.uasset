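; Construction-time track builder that lines a spline with two rows of instanced cones, yellow on one side and blue on the other.
; With a PuntosDT data table, it pairs blue and yellow points by row order and builds SplineCsv2 from their midpoints, repeating the first to close the loop.
; Otherwise it uses PathSpline.
; GenerarConos offsets evenly spaced cones along the right vector; its blue loop is nested inside the yellow, duplicating blue instances.
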(event EventBeginPlay)

(event Collision|EventActorBeginOverlap
  (params (OtherActor :type Actor%20Object%20Reference)))

(fn ConstructionScript
  (Utilities|IsValid (Variables|Default|GetPuntos_DT)
    (:Is%20Valid
      (CallFunction|CsvtoSpline)
      (CallFunction|GenerarConos))
    (:Is%20Not%20Valid
      (CallFunction|GenerarConos))))

(fn GenerarConos
  (Components|InstancedStaticMesh|ClearInstances (Variables|Default|GetISM_ConoAmarillo))
  (Components|InstancedStaticMesh|ClearInstances (Variables|Default|GetISM_ConoAzul))
  (if (Utilities|IsValid (Variables|Default|GetPuntos_DT))
    (Variables|Default|SetSpline_a_usar (Variables|Default|GetSpline_csv2))
    (else
      (Variables|Default|SetSpline_a_usar (Variables|Default|GetPathSpline))))
  (for _index (range 0 (- (Variables|Default|GetNumeroDeConosNaranjas) 1))
    (Components|InstancedStaticMesh|AddInstance (Variables|Default|GetISM_ConoAmarillo) (Math|Transform|MakeTransform (- (Spline|GetLocationatDistanceAlongSpline (Variables|Default|GetSpline_a_usar) (+ (* (Variables|Default|GetSepracionEntreConos) (Math|Conversions|ToFloat(Integer) _index)) 0.01) "Local") (* (Class|SplineComponent|GetRightVectoratDistanceAlongSpline (Variables|Default|GetSpline_a_usar) (+ (* (Variables|Default|GetSepracionEntreConos) (Math|Conversions|ToFloat(Integer) _index)) 0.01) "Local") (Variables|Default|GetSeparacionEntreLineas))) (Spline|GetRotationatDistanceAlongSpline (Variables|Default|GetSpline_a_usar) 0.0 "Local")))
    (for _index_2 (range 0 (- (Variables|Default|GetNumeroDeConosAzules) 1))
      (Components|InstancedStaticMesh|AddInstance (Variables|Default|GetISM_ConoAzul) (Math|Transform|MakeTransform (+ (Spline|GetLocationatDistanceAlongSpline (Variables|Default|GetSpline_a_usar) (+ (* (Variables|Default|GetSepracionEntreConos) (Math|Conversions|ToFloat(Integer) _index_2)) 0.01) "Local") (* (Class|SplineComponent|GetRightVectoratDistanceAlongSpline (Variables|Default|GetSpline_a_usar) (+ (* (Variables|Default|GetSepracionEntreConos) (Math|Conversions|ToFloat(Integer) _index_2)) 0.01) "Local") (Variables|Default|GetSeparacionEntreLineas))) (Spline|GetRotationatDistanceAlongSpline (Variables|Default|GetSpline_a_usar) 0.0 "Local"))))))

(fn CsvtoSpline
  (bind _puntos_dt (Variables|Default|GetPuntos_DT))
  (bind _spline_csv2 (Variables|Default|GetSpline_csv2))
  (Utilities|Array|Clear (Variables|Default|GetPosicionesAzules))
  (Utilities|Array|Clear (Variables|Default|GetPosicionesAmarillos))
  (Spline|ClearSplinePoints (Variables|Default|GetSpline_csv2) true)
  (if (Utilities|IsValid _puntos_dt)
    (bind _outrownames (DataTable|GetDataTableRowNames _puntos_dt))
    (for _array_element _outrownames
      (bind _returnvalue (Utilities|GetDataTableRow _puntos_dt _array_element)
        (:then
          (switch string (.color (Utilities|Struct|Breakcsv_point _returnvalue))
            (:blue
              (Utilities|Array|Add (Variables|Default|GetPosicionesAzules) (Math|Vector|MakeVector (.x (Utilities|Struct|Breakcsv_point _returnvalue)) (.y (Utilities|Struct|Breakcsv_point _returnvalue)) (.z (Utilities|Struct|Breakcsv_point _returnvalue)))))
            (:yellow
              (Utilities|Array|Add (Variables|Default|GetPosicionesAmarillos) (Math|Vector|MakeVector (.x (Utilities|Struct|Breakcsv_point _returnvalue)) (.y (Utilities|Struct|Breakcsv_point _returnvalue)) (.z (Utilities|Struct|Breakcsv_point _returnvalue)))))))))
    (for _index (range 0 (- (Math|Integer|Min(Integer) (Utilities|Array|Length (Variables|Default|GetPosicionesAzules)) (Utilities|Array|Length (Variables|Default|GetPosicionesAmarillos))) 1))
      (Spline|AddSplinePoint (Variables|Default|GetSpline_csv2) (/ (+ (Utilities|Array|Get(acopy) (Variables|Default|GetPosicionesAmarillos) _index) (Utilities|Array|Get(acopy) (Variables|Default|GetPosicionesAzules) _index)) 2.0) "World" true))
    (if (Utilities|IsValid (Variables|Default|GetPuntos_DT))
      (Spline|AddSplinePoint _spline_csv2 (Spline|GetLocationatSplinePoint _spline_csv2 0 "Local") "World" true))))